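; BP_AI_Enemy is an enemy pawn that roams, chases the player and deals contact damage.
; A looping timer moves it to random nearby navigable points; seeing the player via PawnSensing starts a fast follow timer, without clearing the roam timer.
; AttackVolume overlap starts periodic damage to the player, cleared on any end overlap.
; Incoming damage lowers health, destroying it at zero after a delay; its HP widget receives a self reference.
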(event OnSeePawn(PawnSensing)
  (params (Pawn :type Pawn%20Object%20Reference))
  ;[0.05127 0.05127 0.05127] Pawn Sensing
  (if (== Pawn (Game|Player|GetPlayerPawn 0))
    (bind _returnvalue (Utilities|Time|SetTimerbyEvent (delegate Custom|Follow%20Player) 0.001 true))
    (Variables|Default|SetFollow%20Player%20Timer _returnvalue)))

(event OnComponentBeginOverlap(AttackVolume)
  (params (OverlappedComponent :type Primitive%20Component%20Object%20Reference) (OtherActor :type Actor%20Object%20Reference) (OtherComp :type Primitive%20Component%20Object%20Reference) (OtherBodyIndex :type Integer) (bFromSweep :type Boolean) (SweepResult :type Hit%20Result%20Structure%20%28by%20ref%29))
  ;[0.05127 0.05127 0.05127] Apply Damage
  (if (== OtherActor (Game|GetPlayerCharacter 0))
    (bind _returnvalue (Utilities|Time|SetTimerbyEvent (delegate Custom|Damage) 1.0 true))
    (Variables|Default|SetDamage%20Area _returnvalue)))

(event OnComponentEndOverlap(AttackVolume)
  (params (OverlappedComponent :type Primitive%20Component%20Object%20Reference) (OtherActor :type Actor%20Object%20Reference) (OtherComp :type Primitive%20Component%20Object%20Reference) (OtherBodyIndex :type Integer))
  ;[0.05127 0.05127 0.05127] Apply Damage
  (Utilities|Time|ClearandInvalidateTimerbyHandle (Variables|Default|GetDamage%20Area)))

(event Custom|Roam
  ;[0.05127 0.05127 0.05127] Roam
  (bind _randomlocation (Class|NavigationSystemV1|GetRandomLocationinNavigableRadius (Transformation|GetActorLocation) 5e+02 0 0))
  (Rendering|Debug|DrawDebugSphere _randomlocation 5.0 12 "(R=1.000000,G=1.000000,B=1.000000,A=1.000000)" 0.0)
  (AI|AIMoveTo self _randomlocation 0 5.0 false))

(event Custom|Follow%20Player
  ;[0.05127 0.05127 0.05127] Pawn Sensing
  (AI|AIMoveTo self "0, 0, 0" (Game|Player|GetPlayerPawn 0) 2e+02 false
    (:then
      (Variables|/Script/Engine.CharacterMovementComponent|SetMaxWalkSpeed (Variables|Character|GetCharacterMovement) 5e+02))))

(event Custom|Damage
  ;[0.05127 0.05127 0.05127] Apply Damage
  (Game|Damage|ApplyDamage (Game|GetPlayerCharacter 0) 1e+01 0 0))

(event EventBeginPlay
  (Utilities|FlowControl|Sequence
    (:then_0
      ;[0.05127 0.05127 0.05127] Roam
      (bind _returnvalue (Utilities|Time|SetTimerbyEvent (delegate Custom|Roam) 5.0 true))
      (Variables|Default|SetRoam%20Timer _returnvalue))
    (:then_1
      (bind _aswb_enemy_hp (Utilities|Casting|CastToWB_Enemy_HP (UserInterface|GetWidget (Variables|Default|GetHP))))
      (Variables|/Game/MyContent/Widgets/WB_Enemy_HP.WB_Enemy_HP_C|SetPawn _aswb_enemy_hp self)
      (bind _asbp_first_person_character (Utilities|Casting|CastToBP_FirstPersonCharacter (Game|GetPlayerCharacter 0)))
      (Variables|Default|SetAs%20BP%20First%20Person%20Character _asbp_first_person_character))))

(event Game|Damage|EventAnyDamage
  (params (Damage :type Float%20%28single-precision%29) (DamageType :type Damage%20Type%20Object%20Reference) (InstigatedBy :type Controller%20Object%20Reference) (DamageCauser :type Actor%20Object%20Reference))
  ;[0.05127 0.05127 0.05127] Damage Taken
  (Development|PrintString (Utilities|String|ToString(Float) Damage))
  (bind _output_get (Variables|Default|SetHealth (Math|Float|Clamp(Float) (- (Variables|Default|GetHealth) Damage) 0.0 (Variables|Default|GetHealth))))
  (if (<= _output_get 0.0)
    (Utilities|FlowControl|Delay 1.0)
    (Actor|DestroyActor)))

(fn ConstructionScript)