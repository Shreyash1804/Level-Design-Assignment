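; Smart enemy AI actor that patrols a looping list of locations with random pauses and chases the player on sight.
; Pawn sensing triggers a one-time sprint and turn toward the player; a retriggerable delay resumes slow patrol once sightings stop.
; Damage lowers health, updates a widget health bar rotated toward the player only at BeginPlay, and destroys the actor at zero.
; Bullet-firing logic exists but is disconnected.
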(event OnSeePawn(PawnSensing)
  (params (Pawn :type Pawn%20Object%20Reference))
  ;[0.05127 0.05127 0.05127] Pawn Sensing
  (if (== Pawn (Variables|Default|GetPlayer%20Character))
    (Utilities|FlowControl|Sequence
      (:then_0
        (Utilities|FlowControl|DoOnce false
          (:Completed
            (Variables|/Script/Engine.CharacterMovementComponent|SetMaxWalkSpeed (Variables|Character|GetCharacterMovement) 5e+02)
            (Transformation|SetActorRotation self (Math|Rotator|FindLookatRotation (Transformation|GetActorLocation) (Transformation|GetActorLocation (Variables|Default|GetPlayer%20Character)))))))
      (:then_1
        (AI|AIMoveTo self "0, 0, 0" (Variables|Default|GetPlayer%20Character) 5.0 false
          (:then
            (Utilities|FlowControl|RetriggerableDelay 2.0)
            (Variables|/Script/Engine.CharacterMovementComponent|SetMaxWalkSpeed (Variables|Character|GetCharacterMovement) 1.5e+02)
            (CallFunction|SprintAgain)
            (CallFunction|GuardPatrol))))
      (:then_2
        (if (Variables|Default|GetShootDelay)
          _)))))

(event Custom|Guard%20Patrol
  ;[0.05127 0.05127 0.05127] Patroling
  (Variables|/Script/Engine.CharacterMovementComponent|SetMaxWalkSpeed (Variables|Character|GetCharacterMovement) 1.5e+02)
  (AI|AIMoveTo self (Utilities|Array|Get(acopy) (Variables|Default|GetPatrolLocation) (Variables|Default|GetLocations)) 0 5.0 false
    (:OnSuccess
      (Utilities|FlowControl|Delay (Math|Random|RandomFloatinRange 1.0 2.0))
      (CallFunction|GuardPatrol)
      (Math|Integer|IncrementInt (Variables|Default|GetLocations)
        (:%20%20
          (if (== (Variables|Default|GetLocations) (Variables|Default|GetNo%20of%20Patrol%20Locations))
            (Variables|Default|SetLocations 0)))))))

(event Custom|SprintAgain
  ;[0.05127 0.05127 0.05127] Pawn Sensing
  (Utilities|FlowControl|DoOnce false) ; enters at Reset
)

(event EventBeginPlay
  ;[0.05127 0.05127 0.05127] BeginPlay
  (Utilities|FlowControl|Sequence
    (:then_0
      (CallFunction|GuardPatrol)
      (Variables|Default|SetNo%20of%20Patrol%20Locations (Utilities|Array|Length (Variables|Default|GetPatrolLocation))))
    (:then_1
      (Variables|Default|SetPlayer%20Character (Game|GetPlayerCharacter 0)))
    (:then_2
      (bind _aswb_smart_enemy_hp (Utilities|Casting|CastToWB_SmartEnemy_HP (UserInterface|GetWidget (Variables|Default|GetHealth%20Bar%20Widget))))
      (Variables|Default|SetAs%20WB%20Smart%20Enemy%20HP _aswb_smart_enemy_hp)
      (Variables|/Script/UMG.ProgressBar|SetPercent (Variables|/Game/MyContent/Widgets/WB_SmartEnemy_HP.WB_SmartEnemy_HP_C|GetHealthBar _aswb_smart_enemy_hp) (/ (Variables|Default|GetHealth) 1e+02)))
    (:then_3
      (Transformation|SetWorldRotation (Variables|Default|GetHealth%20Bar%20Widget) (Math|Rotator|FindLookatRotation (Transformation|GetWorldLocation (Variables|Default|GetHealth%20Bar%20Widget)) (Transformation|GetWorldLocation (Variables|/Script/Engine.Actor|GetRootComponent (Variables|Default|GetPlayer%20Character)))) false false))))

(event Game|Damage|EventAnyDamage
  (params (Damage :type Float%20%28single-precision%29) (DamageType :type Damage%20Type%20Object%20Reference) (InstigatedBy :type Controller%20Object%20Reference) (DamageCauser :type Actor%20Object%20Reference))
  ;[0.05127 0.05127 0.05127] Damage Taken
  (Development|PrintString (Utilities|String|ToString(Float) Damage))
  (bind _output_get (Variables|Default|SetHealth (Math|Float|Clamp(Float) (- (Variables|Default|GetHealth) Damage) 0.0 (Variables|Default|GetHealth))))
  (Development|PrintString (Utilities|String|ToString(Float) _output_get))
  (Variables|/Script/UMG.ProgressBar|SetPercent (Variables|/Game/MyContent/Widgets/WB_SmartEnemy_HP.WB_SmartEnemy_HP_C|GetHealthBar (Variables|Default|GetAs%20WB%20Smart%20Enemy%20HP)) (/ (Variables|Default|GetHealth) 1e+02))
  (if (<= (Variables|Default|GetHealth) 0.0)
    (Utilities|FlowControl|Delay 1.0)
    (Actor|DestroyActor)))

(fn ConstructionScript)