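; Shooter enemy AI that walks between patrol points, pausing randomly at each, and attacks the player when seen.
; Pawn sensing triggers a sprint and chase, fires BP_Bullet from the weapon muzzle on a short cooldown, and uses a retriggerable delay to resume patrol.
; Damage lowers Health and enables mesh physics at zero, while sphere overlaps damage BP_AI_Enemy actors.
; Health bar update and facing logic exists but never runs.
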(event OnComponentBeginOverlap(Sphere)
  (params (OverlappedComponent :type Primitive%20Component%20Object%20Reference) (OtherActor :type Actor%20Object%20Reference) (OtherComp :type Primitive%20Component%20Object%20Reference) (OtherBodyIndex :type Integer) (bFromSweep :type Boolean) (SweepResult :type Hit%20Result%20Structure%20%28by%20ref%29))
  ;[0.05127 0.05127 0.05127] Apply Damage
  (bind _asbp_ai_enemy (Utilities|Casting|CastToBP_AI_Enemy OtherActor))
  (Game|Damage|ApplyDamage _asbp_ai_enemy 2e+01 0 0))

(event OnSeePawn(PawnSensing)
  (params (Pawn :type Pawn%20Object%20Reference))
  (bind _weapon (Variables|Default|GetWeapon))
  (bind _returnvalue (Transformation|GetSocketTransform _weapon "b_gun_muzzleflash" "RTS_World"))
  ;[0.05127 0.05127 0.05127] Pawn Sensing
  (if (== Pawn (Variables|Default|GetPlayer%20Character))
    (Utilities|FlowControl|Sequence
      (:then_0
        (Utilities|FlowControl|DoOnce false
          (:Completed
            (Variables|/Script/Engine.CharacterMovementComponent|SetMaxWalkSpeed (Variables|Character|GetCharacterMovement) 5e+02)
            (Transformation|SetActorRotation self (Math|Rotator|FindLookatRotation (Transformation|GetActorLocation) (Transformation|GetActorLocation (Variables|Default|GetPlayer%20Character)))))))
      (:then_1
        (AI|AIMoveTo self "0, 0, 0" (Variables|Default|GetPlayer%20Character) 5.0 false
          (:then
            (Utilities|FlowControl|RetriggerableDelay 2.0)
            (Variables|/Script/Engine.CharacterMovementComponent|SetMaxWalkSpeed (Variables|Character|GetCharacterMovement) 1.5e+02)
            (CallFunction|SprintAgain)
            (CallFunction|GuardPatrol))))
      (:then_2
        (if (Variables|Default|GetShootDelay)
          (Game|SpawnActorfromClass "/Game/MyContent/Blueprints/BP_Bullet.BP_Bullet_C" (Math|Transform|MakeTransform (.location _returnvalue) (Math|Rotator|MakeRotator (.roll (.rotation _returnvalue)) (.pitch (.rotation _returnvalue)) (+ (.yaw (.rotation _returnvalue)) 9e+01)) "1.000000,1.000000,1.000000") "Undefined" "MultiplyWithRoot" 0 0)
          (Variables|Default|SetShootDelay false)
          (Utilities|FlowControl|Delay 0.2)
          (Variables|Default|SetShootDelay true))))))

(event Custom|Guard%20Patrol
  ;[0.05127 0.05127 0.05127] Patroling
  (Variables|/Script/Engine.CharacterMovementComponent|SetMaxWalkSpeed (Variables|Character|GetCharacterMovement) 1.5e+02)
  (AI|AIMoveTo self (Utilities|Array|Get(acopy) (Variables|Default|GetPatrolLocation) (Variables|Default|GetLocations)) 0 5.0 false
    (:OnSuccess
      (Utilities|FlowControl|Delay (Math|Random|RandomFloatinRange 1.0 2.0))
      (CallFunction|GuardPatrol)
      (Math|Integer|IncrementInt (Variables|Default|GetLocations)
        (:%20%20
          (if (== (Variables|Default|GetLocations) (Variables|Default|GetNo%20of%20Patrol%20Locations))
            (Variables|Default|SetLocations 0)))))))

(event Custom|SprintAgain
  ;[0.05127 0.05127 0.05127] Pawn Sensing
  (Utilities|FlowControl|DoOnce false) ; enters at Reset
)

(event Game|Damage|EventAnyDamage
  (params (Damage :type Float%20%28single-precision%29) (DamageType :type Damage%20Type%20Object%20Reference) (InstigatedBy :type Controller%20Object%20Reference) (DamageCauser :type Actor%20Object%20Reference))
  (bind _mesh (Variables|Character|GetMesh))
  ;[0.05127 0.05127 0.05127] Damage Taken
  (bind _output_get (Variables|Default|SetHealth (Math|Float|Clamp(Float) (- (Variables|Default|GetHealth) Damage) 0.0 (Variables|Default|GetHealth))))
  (if (<= _output_get 0.0)
    (Physics|SetSimulatePhysics _mesh true)
    (Class|SkeletalMeshComponent|SetPhysicsBlendWeight _mesh 0.0)
    (Collision|SetCollisionEnabled _mesh "QueryAndPhysics")))

(event EventBeginPlay
  ;[0.05127 0.05127 0.05127] BeginPlay
  (Utilities|FlowControl|Sequence
    (:then_0
      (CallFunction|GuardPatrol)
      (Variables|Default|SetNo%20of%20Patrol%20Locations (Utilities|Array|Length (Variables|Default|GetPatrolLocation))))
    (:then_1
      (Variables|Default|SetPlayer%20Character (Game|GetPlayerCharacter 0)))
    (:then_2)
    (:then_3)))

(fn ConstructionScript)